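; BP_Player is the player character, which moves, jumps and collects coins.
; Legacy axis inputs drive movement relative to the control rotation, using yaw for forward and yaw plus roll for right.
; The jump action starts and stops the built-in character jump.
; On actor overlap, it casts the other actor to BP_Coin and calls GetCoin, leaving pickup handling to the coin.
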(event `InputAxis|Movimiento adelante y atras`
  (params (AxisValue :type "Float (single-precision)"))
  (bind (_returnvalue_roll _returnvalue_pitch _returnvalue_yaw) (`KismetMathLibrary.BreakRotator` (`self.GetControlRotation`)))
  (`self.AddMovementInput` (`KismetMathLibrary.GetForwardVector` (`KismetMathLibrary.MakeRotator` 0.0 0.0 _returnvalue_yaw)) AxisValue))

(event `InputAction|Salto`
  (params (Key :type "Key Structure"))
  (:`Pressed`
    (`self.Jump`))
  (:`Released`
    (`self.StopJumping`)))

(event `InputAxis|Movimiento izquierda y derecha`
  (params (AxisValue :type "Float (single-precision)"))
  (bind (_returnvalue_roll _returnvalue_pitch _returnvalue_yaw) (`KismetMathLibrary.BreakRotator` (`self.GetControlRotation`)))
  (`self.AddMovementInput` (`KismetMathLibrary.GetRightVector` (`KismetMathLibrary.MakeRotator` _returnvalue_roll 0.0 _returnvalue_yaw)) AxisValue))

(event `self.ReceiveActorBeginOverlap`
  (params (OtherActor :type "Actor Object Reference"))
  (bind _asbp_coin (cast `/Game/Coin/BP_Coin` OtherActor))
  (`/Game/Coin/BP_Coin.GetCoin` _asbp_coin))

(fn `UserConstructionScript`)